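; BP_Ball01 is a player-controlled rolling ball with a jump.
; UpDown and LeftRight axis inputs, scaled by Multiply, apply angular acceleration to the Sphere around Y and X respectively.
; SpaceBar restarts the Jump timeline, which each update sets the Sphere's world position to the current actor location plus a scaled vertical curve offset, rather than applying an impulse.
; No ground check gates the jump.
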(event `InputAxis|UpDown`
  (params (AxisValue :type "Float (single-precision)"))
  (`PrimitiveComponent.AddTorqueInDegrees` (`self.Sphere`) (`KismetMathLibrary.MakeVector` 0.0 (* AxisValue (`self.Multiply`))) "None" true))

(event `InputAxis|LeftRight`
  (params (AxisValue :type "Float (single-precision)"))
  (`PrimitiveComponent.AddTorqueInDegrees` (`self.Sphere`) (`KismetMathLibrary.MakeVector` (* AxisValue (`self.Multiply`))) "None" true))

(event `Key|SpaceBar`
  (params (Key :type "Key Structure"))
  (bind (_returnvalue_x _returnvalue_y _returnvalue_z) (`KismetMathLibrary.BreakVector` (`self.K2_GetActorLocation`)))
  (:`Pressed`
    (bind (_direction _jump) (`Timeline|Jump` :!via `PlayFromStart`)
      (:`Update`
        (`SceneComponent.K2_SetWorldLocation` (`self.Sphere`) (`KismetMathLibrary.MakeVector` _returnvalue_x _returnvalue_y (+ (* (.z _jump) 15.0) _returnvalue_z)) false false)))))

(fn `UserConstructionScript`)