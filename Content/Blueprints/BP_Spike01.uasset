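; BP_Spike01 is a spike hazard that restarts the current level when anything overlaps its capsule.
; On begin play, a timeline drives the point light's intensity between SpikeLight and zero through its SpikeFlicker track.
; On overlap, with no check on the actor, the camera fades to dark red and holds, then the current level reopens by name after a short delay.
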(event `self.ReceiveBeginPlay`
  (bind (_direction _spikeflicker) (`Timeline|Timeline_0`)
    (:`Update`
      (`LightComponent.SetIntensity` (`self.PointLight`) (`KismetMathLibrary.Lerp` (`self.SpikeLight`) 0.0 _spikeflicker)))))

(event `self.Capsule.OnComponentBeginOverlap`
  (params (OverlappedComponent :type "PrimitiveComponent Object Reference") (OtherActor :type "Actor Object Reference") (OtherComp :type "PrimitiveComponent Object Reference") (OtherBodyIndex :type Integer) (bFromSweep :type Boolean) (SweepResult :type "HitResult Structure (by ref)"))
  (bind _returnvalue (`GameplayStatics.GetCurrentLevelName` true))
  (`PlayerCameraManager.StartCameraFade` (`PlayerController.PlayerCameraManager` (`GameplayStatics.GetPlayerController` 0)) 0.0 1.0 1.0 (struct :`R` 0.307292 :`G` 0.006876 :`A` 1.0) false true)
  (`KismetSystemLibrary.Delay` 1.0)
  (`GameplayStatics.OpenLevel` (`KismetStringLibrary.Conv_StringToName` _returnvalue)))

(fn `UserConstructionScript`)