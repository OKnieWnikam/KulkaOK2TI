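; BP_Flower01 is a spinning pickup-style actor with a point light that flies to the player and disappears when its sphere is overlapped.
; Tick applies a constant yaw spin, and any sphere overlap plays the TL_CrystalMove timeline without filtering the overlapping actor.
; The timeline lerps from the actor's current location to player pawn 0's live position, so it homes in, while a flicker track drives light intensity.
; The actor destroys itself when the timeline finishes.
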(event `self.Sphere.OnComponentBeginOverlap`
  (params (OverlappedComponent :type "PrimitiveComponent Object Reference") (OtherActor :type "Actor Object Reference") (OtherComp :type "PrimitiveComponent Object Reference") (OtherBodyIndex :type Integer) (bFromSweep :type Boolean) (SweepResult :type "HitResult Structure (by ref)"))
  (bind (_direction _movement _crystal_flicker) (`Timeline|TL_CrystalMove`)
    (:`Update`
      (`self.K2_SetActorLocation` (`KismetMathLibrary.VLerp` (`self.K2_GetActorLocation`) (`self.K2_GetActorLocation` (`GameplayStatics.GetPlayerPawn` 0)) _movement))
      (`LightComponent.SetIntensity` (`self.PointLight`) (`KismetMathLibrary.Lerp` (`self.Crystal  Light Intencity`) 0.0 _crystal_flicker)))
    (:`Finished`
      (`self.K2_DestroyActor`))))

(event `self.ReceiveTick`
  (params (DeltaSeconds :type "Float (single-precision)"))
  (`self.K2_AddActorLocalRotation` (`KismetMathLibrary.MakeRotator` 0.0 0.0 (* DeltaSeconds (`self.Yaw Per Second`)))))

(fn `UserConstructionScript`)